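; Networked game state that resolves the end of a match between Blue and Red teams and shows the result on screen.
; An event casts each player state, triggering the lost reaction on Blue avatars and the won reaction on Red ones.
; It then creates a results widget showing a loss message for a local Blue player, otherwise the winning player's nickname.
; A second event removes that widget.
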(event Custom|CustomEvent
  (for _array_element (Variables|Default|GetPlayerArray)
    (bind _asnet_player_state (Utilities|Casting|CastToNetPlayerState _array_element))
    (switch Utilities|FlowControl|Switch|SwitchonEPlayerTeam (.teamid (Variables|/Script/Laabwork43.NetPlayerState|GetData _asnet_player_state))
      (:TEAM_Blue
        (Default|OnPlayerLost (.AsMy%20Net%20Avatar (Utilities|Casting|CastToMyNetAvatar (Variables|/Script/Engine.PlayerState|GetPawnPrivate _asnet_player_state)))))
      (:TEAM_Red
        (Default|OnPlayerWon (.AsMy%20Net%20Avatar (Utilities|Casting|CastToMyNetAvatar (Variables|/Script/Engine.PlayerState|GetPawnPrivate _asnet_player_state)))))))
  (CallFunction|ShowResultMessage))

(event Custom|CustomEvent_1
  (Widget|RemovefromParent (Variables|Default|GetMessage%20Widget)))

(fn ConstructionScript)

(fn ShowResultMessage
  (bind _returnvalue (Class|NetGameState|GetPlayerStatebyIndex (Variables|Default|GetWinningPlayer)))
  (bind _returnvalue_2 (UserInterface|CreateWidget "/Game/Blueprints/UMG/W_GameResults.W_GameResults_C" 0 (select (Utilities|Enum|Equal(Enum) (.teamid (Variables|/Script/Laabwork43.NetPlayerState|GetData (.AsNet%20Player%20State (Utilities|Casting|CastToNetPlayerState (Variables|/Script/Engine.Controller|GetPlayerState (Game|GetPlayerController 0)))))) "TEAM_Blue") "YOU LOSE" (Utilities|Text|FormatText "{Name} WINS!" (.Nickname (Utilities|Struct|BreakSPlayerInfo (Variables|/Script/Laabwork43.NetPlayerState|GetData _returnvalue)))))))
  (bind _output_get (Variables|Default|SetMessage%20Widget _returnvalue_2))
  (UserInterface|Viewport|AddtoViewport _output_get 0))